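; BP_Enemy is a sprite-based enemy that teleports to a fixed fight position and shows its HP widget when the player overlaps it.
; An enemy ID selects a data asset for animation, HP, firepower and boss setup.
; Damage flashes the sprite red and updates HP, destroying the enemy at zero; bosses can recover HP.
; Tick locks rotation, and a MOVE event requests AI pathing toward the player.
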(event `self.ReceiveTick`
  (params (DeltaSeconds :type "Float (single-precision)"))
  (`self.K2_SetActorRotation` (struct)))

(event `self.ReceiveBeginPlay`
  ;[1 1 1] BSP
  (bind _asabp_enemy (cast `/Game/blueprint/ABP/ABP_Enemy` (`self.GetAnimInstance`)))
  (set `self.As ABP Enemy` _asabp_enemy)
  (`self.Init_enemy` (`self.Enemy ID`)))

(event `self.CapsuleComponent.OnComponentBeginOverlap`
  (params (OverlappedComponent :type "PrimitiveComponent Object Reference") (OtherActor :type "Actor Object Reference") (OtherComp :type "PrimitiveComponent Object Reference") (OtherBodyIndex :type Integer) (bFromSweep :type Boolean) (SweepResult :type "HitResult Structure (by ref)"))
  ;[1 1 1] tp to fight field
  (if (`self.ActorHasTag` OtherActor "player")
    (`self.K2_TeleportTo` (136.0 1660.0 0.1))
    (`self.UDH Enemy`)))

(event `/Game/blueprint/interfaces/Enemy.Received attack`
  (params (damage :type "Float (double-precision)"))
  ;[1 1 1] attacted sound and effect
  (`PaperFlipbookComponent.SetSpriteColor` (`self.Sprite`) (struct :`R` 1.0 :`A` 1.0))
  (`GameplayStatics.PlaySound2D` "/Game/sounds/soundscape/attack_hit.attack_hit" 1.0 1.0 0.0 null null)
  (bind _returnvalue (`self.HP_calculation` damage))
  (if _returnvalue
    (`KismetSystemLibrary.PrintString` "victory")
    (set `self.Status` "NewEnumerator1")
    (`KismetSystemLibrary.Delay` 0.2)
    (`self.K2_DestroyActor`)
    (`Widget.RemoveFromParent` (`self.UI_Enemy`))
    (else
      (`KismetSystemLibrary.Delay` 0.2)
      (`PaperFlipbookComponent.SetSpriteColor` (`self.Sprite`) (struct :`R` 1.0 :`G` 1.0 :`B` 1.0 :`A` 1.0)))))

(event `MOVE`
  (bind _returnvalue (`GameplayStatics.GetPlayerPawn` 0))
  (`/Engine/EditorBlueprintResources/StandardMacros.IsValid` _returnvalue
    (:`Is Valid`
      (`|AIMoveTo` self (0.0 0.0 0.0) _returnvalue
        (:`OnSuccess`
          (`KismetSystemLibrary.K2_ClearAndInvalidateTimerHandle` (`self.Pathfinding timer`)))
        (:`OnFail`
          (bind _returnvalue_2 (`KismetSystemLibrary.K2_SetTimerDelegate` (`|CreateDelegate` :!event `MOVE`) 0.5 true))
          (set `self.Pathfinding timer` _returnvalue_2))))))

(event `/Game/blueprint/interfaces/Enemy.boss1_recover`
  (bind _returnvalue (`KismetMathLibrary.FClamp` (+ (`self.HP`) 20.0) 0.0 200.0))
  ;[1 1 1] boss1_recover
  (if (`self.boss?`)
    (set `self.HP` _returnvalue)
    (`KismetSystemLibrary.PrintString` (`KismetStringLibrary.Conv_DoubleToString` _returnvalue))
    (`self.HP Udpdate` 0.0)))

(fn `dead`
  (returns (status :type Boolean))
  (return (`|EnumEquality` (`self.status`) "NewEnumerator1")))

(fn `Enemy Attributes`
  (params (HP :type "Float (double-precision)") (Firepower :type "Float (double-precision)"))
  (set `self.Firepower` Firepower))

(fn `HP Udpdate`
  (params (HP :type "Float (double-precision)"))
  (`/Game/UI/UI_enemy.Update_HP_enemy` (`self.UI_Enemy`) (`self.HP`) (`/Game/Data_assets/Enemy_Data_Assets/DA_Enemy.HPmax` (`self.Enemy_data`)))
  (`/Game/UI/UI_enemy.Update_HP_Enemy_prograss` (`self.UI_Enemy`) (`self.HP`) (`/Game/Data_assets/Enemy_Data_Assets/DA_Enemy.HPmax` (`self.Enemy_data`))))

(fn `Hp_calculation`
  (params (damage_value :type "Float (double-precision)"))
  (returns (ReturnValue :type Boolean))
  (set `self.HP` (- (`self.HP`) damage_value))
  (`self.HP Udpdate` (`self.HP`))
  (`KismetSystemLibrary.PrintString` (`KismetStringLibrary.Conv_DoubleToString` (`self.HP`)))
  (return (<= (`self.HP`) 0.0)))

(fn `Init_enemy`
  (params (`enemy id` :type "/Game/blueprint/enumeration/Enemy_ID Enum" :default "NewEnumerator0"))
  (bind _enemy_data (`self.Enemy_data`))
  (bind _as_abp_enemy (`self.As ABP Enemy`))
  (switch `/Game/blueprint/enumeration/Enemy_ID` `enemy id`
    (:`NewEnumerator0`
      (bind _output_get (set `self.Enemy_data` "/Game/Data_assets/Enemy_Data_Assets/DA_bamboo.DA_bamboo"))
      (set `/Game/blueprint/ABP/ABP_Enemy.Enemy movement animation` (`/Game/Data_assets/Enemy_Data_Assets/DA_Enemy.picture` _output_get) _as_abp_enemy))
    (:`NewEnumerator1`
      (bind _output_get_2 (set `self.Enemy_data` "/Game/Data_assets/Enemy_Data_Assets/DA_bugger.DA_bugger"))
      (set `/Game/blueprint/ABP/ABP_Enemy.Enemy movement animation` (`/Game/Data_assets/Enemy_Data_Assets/DA_Enemy.picture` _output_get_2) _as_abp_enemy))
    (:`NewEnumerator3`
      (bind _output_get_3 (set `self.Enemy_data` "/Game/Data_assets/Enemy_Data_Assets/DA_boss1.DA_boss1"))
      (set `/Game/blueprint/ABP/ABP_Enemy.Enemy movement animation` (`/Game/Data_assets/Enemy_Data_Assets/DA_Enemy.picture` _output_get_3) _as_abp_enemy)
      (`CapsuleComponent.SetCapsuleRadius` (`self.CapsuleComponent`) 70.0 true)
      (set `self.boss?` (`/Game/Data_assets/Enemy_Data_Assets/DA_Enemy.boss?` _enemy_data))))
  (set `self.HP` (`/Game/Data_assets/Enemy_Data_Assets/DA_Enemy.HP` _enemy_data))
  (`self.Enemy Attributes` (`self.HP`) (`/Game/Data_assets/Enemy_Data_Assets/DA_Enemy.firepower` _enemy_data))
  (set `self.pre-transport position` (`self.K2_GetActorLocation`)))

(fn `UDH Enemy`
  (bind _returnvalue (`|CreateWidget` "/Game/UI/UI_enemy.UI_enemy_C"))
  (bind _output_get (set `self.UI_Enemy` _returnvalue))
  (`UserWidget.AddToViewport` _output_get 0)
  (`self.HP Udpdate` (`self.HP`)))

(fn `UserConstructionScript`)