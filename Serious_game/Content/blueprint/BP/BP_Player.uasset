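; Player character with a sprite, Enhanced Input movement, NPC dialog via BPI_dialog, and quiz-based combat.
; Touching an Enemy-tagged actor teleports the player to a fight field and opens UI_Fight, where correct answers hit the enemy and wrong or empty ones hurt the player.
; BackTp returns the player with a knockback and triggers prop spawning.
; Stats load from PlayerData and feed the HUD, with coin-driven exponential leveling and hotkeyed healing or timed-buff items.
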(event `self.ReceiveBeginPlay`
  (bind _player_data (`self.Player_data`))
  ;[1 1 1] BSP
  (`self.Player Attributes` (`/Game/Data_assets/Player_Data_Assets/DA_Character.Experience` _player_data) (`/Game/Data_assets/Player_Data_Assets/DA_Character.Experience points required to upgrade` _player_data) (`/Game/Data_assets/Player_Data_Assets/DA_Character.grade` _player_data) (`KismetMathLibrary.Conv_IntToDouble` (`/Game/Data_assets/Player_Data_Assets/DA_Character.money` _player_data)) (`/Game/Data_assets/Player_Data_Assets/DA_Character.HP` _player_data) (`/Game/Data_assets/Player_Data_Assets/DA_Character.firepower` _player_data))
  (`self.HUD_initialize`))

(event `EnhancedInput|/Game/Enhanced_inputs/IA_Move`
  (params (ActionValue :type "Vector2D Structure") (ElapsedSeconds :type "Float (double-precision)") (TriggeredSeconds :type "Float (double-precision)") (InputAction :type "InputAction Object Reference" :default "/Game/Enhanced_inputs/IA_Move.IA_Move"))
  (bind (_x _y) (`KismetMathLibrary.BreakVector2D` ActionValue))
  ;[1 1 1] MOVE
  (:`Triggered`
    (set `self.X` _x)
    (set `self.Y` _y)
    (`self.AddMovementInput` (1.0 0.0 0.0) (`self.X`))
    (`self.AddMovementInput` (0.0 1.0 0.0) (`self.Y`))))

(event `self.CapsuleComponent.OnComponentBeginOverlap`
  (params (OverlappedComponent :type "PrimitiveComponent Object Reference") (OtherActor :type "Actor Object Reference") (OtherComp :type "PrimitiveComponent Object Reference") (OtherBodyIndex :type Integer) (bFromSweep :type Boolean) (SweepResult :type "HitResult Structure (by ref)"))
  (bind _ui_fight (`self.UI Fight`))
  ;[1 1 1] tp to fight field
  (set `self.location` (`self.K2_GetActorLocation` self))
  (set `self.Enemy Location` (`self.K2_GetActorLocation` OtherActor))
  (set `self.current enemy` OtherActor)
  (if (`self.ActorHasTag` OtherActor "Enemy")
    (`self.K2_TeleportTo` (28.0 1670.0 0.1))
    (if (`|EnumEquality` (`Widget.Visibility` _ui_fight) "Visible")
      (bind _returnvalue (`|CreateWidget` "/Game/UI/UI_Fight.UI_Fight_C" null "/Game/Data_assets/Question_data_assets/DA_question.DA_question" null null))
      (bind _output_get (set `self.UI Fight` _returnvalue))
      (`SceneComponent.K2_SetRelativeLocation` (`self.Camera`) (0.0 50.0 0.0) false false)
      (else
        (`Widget.SetVisibility` _ui_fight "Visible")))
    (`self.DisableInput` (`CharacterMovementComponent.GetCharacterOwner` (`self.CharacterMovement`)) null)
    (`UserWidget.AddToViewport` _output_get 0)
    (bind _foundwidgets (`WidgetBlueprintLibrary.GetAllWidgetsOfClass` "/Game/UI/UI_Fight.UI_Fight_C"))
    (message `/Game/blueprint/interfaces/Enemy.set enemy` (`|GetArrayItem` _foundwidgets) (cast `/Game/blueprint/BP/BP_Enemy` (`self.current enemy`) :!pure true))))

(event `/Game/blueprint/interfaces/Enemy.Received attack`
  (params (damage :type "Float (double-precision)"))
  ;[1 1 1] attacted sound and effect
  (`PaperFlipbookComponent.SetSpriteColor` (`self.Sprite`) (struct :`R` 1.0 :`A` 1.0))
  (`GameplayStatics.PlaySound2D` "/Game/sounds/soundscape/attack_hit.attack_hit" 1.0 1.0 0.0 null null)
  (`self.HP_calculation` damage)
  (`self.Update_HP`)
  (`KismetSystemLibrary.Delay` 0.2)
  (`PaperFlipbookComponent.SetSpriteColor` (`self.Sprite`) (struct :`R` 1.0 :`G` 1.0 :`B` 1.0 :`A` 1.0))
  (message `/Game/blueprint/interfaces/Enemy.boss1_recover` (`self.current enemy`)))

(event `/Game/blueprint/interfaces/player.back tp`
  (params (judge :type Boolean))
  ;[1 1 1] back tp after fight
  (if judge
    (`self.K2_TeleportTo` :`self` self :`DestLocation` (`self.location`))
    (`self.LaunchCharacter` self (* 200 (`KismetMathLibrary.GetDirectionUnitVector` (`self.Enemy Location`) (`self.location`))) true false)
    (`KismetSystemLibrary.Delay` 0.2)
    (`/Game/blueprint/instances/object_management.Setting up props pool` (`/Game/blueprint/instances/Game_instances.object management` (`/Game/blueprint/instances/Public_Blueprints_Library.get Game_instances`)) (`self.Enemy Location`))
    (`self.EnableInput` (`CharacterMovementComponent.GetCharacterOwner` (`self.CharacterMovement`)) null)))

(event `/Game/blueprint/interfaces/Items.Get_item`
  (params (`Type of items` :type "/Game/blueprint/enumeration/Enumeration_of_props/Props_classification Enum" :default "NewEnumerator0"))
  ;[1 1 1] add items number
  (switch `/Game/blueprint/enumeration/Enumeration_of_props/Props_classification` `Type of items`
    (:`NewEnumerator0`
      (`self.add_EXP`))
    (:`NewEnumerator1`
      (`self.Update number of item1` 1))
    (:`NewEnumerator2`
      (`self.Update number of item2` 1))
    (:`NewEnumerator3`
      (`self.Update number of item3` 1))))

(event `/Game/blueprint/interfaces/Items.Medical kit function`
  ;[1 1 1] Prop function
  (set `self.HP` (+ (`self.HP`) 20.0))
  (`self.Update_HP`))

(event `Key|One`
  (params (Key :type "Key Structure"))
  ;[1 1 1] Use items number
  (:`Pressed`
    (`self.Update number of item1` 0)
    (`KismetSystemLibrary.PrintString` "1")
    (`/Game/blueprint/interfaces/Items.Beef Effect`)))

(event `Key|Two`
  (params (Key :type "Key Structure"))
  ;[1 1 1] Use items number
  (:`Pressed`
    (`self.Update number of item2` 0)
    (`KismetSystemLibrary.PrintString` "2")
    (`/Game/blueprint/interfaces/Items.Medical kit function`)))

(event `/Game/blueprint/interfaces/Items.Reel effect`
  ;[1 1 1] Prop function
  (set `self.Firepower` (+ (`self.Firepower`) 50.0))
  (`KismetSystemLibrary.Delay` 10.0)
  (set `self.Firepower` (- (`self.Firepower`) 50.0)))

(event `Key|Three`
  (params (Key :type "Key Structure"))
  ;[1 1 1] Use items number
  (:`Pressed`
    (`self.Update number of item3` 0)
    (`KismetSystemLibrary.PrintString` "3")
    (`/Game/blueprint/interfaces/Items.Reel effect`)))

(event `/Game/blueprint/interfaces/Items.Beef Effect`
  ;[1 1 1] Prop function
  (set `self.HP` (+ (`self.HP`) 50.0))
  (`self.Update_HP`)
  (`KismetSystemLibrary.Delay` 10.0)
  (set `self.HP` (- (`self.HP`) 50.0))
  (`self.Update_HP`))

(event `Key|F`
  (params (Key :type "Key Structure"))
  ;[1 1 1] dialog
  (:`Pressed`
    (for _array_element (`self.GetOverlappingActors` "/Game/NPC/NPC_BP/NPC1.NPC1_C")
      (if (`KismetSystemLibrary.DoesImplementInterface` _array_element "/Game/NPC/NPC_BP/BPI_dialog.BPI_dialog_C")
        (message `/Game/NPC/NPC_BP/BPI_dialog.Talk` _array_element)))))

(event `/Game/blueprint/interfaces/Enemy.answer check`
  (params (NewParam :type "/Game/blueprint/enumeration/playeroption_status Enum" :default "NewEnumerator0"))
  ;[1 1 1] call attack
  (switch `/Game/blueprint/enumeration/playeroption_status` NewParam
    (:`NewEnumerator0`
      (message `/Game/blueprint/interfaces/Enemy.Received attack` (`self.current enemy`) (`self.Firepower`)))
    (:`NewEnumerator1`
      (message `/Game/blueprint/interfaces/Enemy.Received attack` self (`/Game/blueprint/BP/BP_Enemy.Firepower` (cast `/Game/blueprint/BP/BP_Enemy` (`self.current enemy`) :!pure true)) :!label _label))
    (:`NewEnumerator2`
      (goto _label))))

(fn `add_EXP`
  (locals (`more EXP` :type "Float (double-precision)"))
  (set `self.EXP` (+ (`self.EXP`) (`self.Money`)))
  (while (>= (`self.EXP`) (`self.EXP to update`))
    (set `local.more EXP` (- (`self.EXP`) (`self.EXP to update`)))
    (`/Engine/EditorBlueprintResources/StandardMacros.IncrementInt` (`self.Grade`)
      (:`  `
        (`self.Update_EXP_Standard`)
        (set `self.EXP` (`local.more EXP`)))))
  (`self.Update_EXP`))

(fn `HP_calculation`
  (params (damage_value :type "Float (double-precision)"))
  (returns (ReturnValue :type Boolean))
  (bind _output_get (set `self.HP` (`KismetMathLibrary.FClamp` (- (`self.HP`) damage_value) 0.0 (`self.HP`))))
  (return (== _output_get 0.0)))

(fn `HUD_initialize`
  (bind _returnvalue (`|CreateWidget` "/Game/UI/UI_state.UI_state_C"))
  (bind _output_get (set `self.UI_state` _returnvalue))
  (`UserWidget.AddToViewport` _output_get 0)
  (`self.Update_EXP`)
  (`self.Update_HP`))

(fn `Player Attributes`
  (params (EXP :type "Float (double-precision)") (`EXP to update` :type "Float (double-precision)") (grade :type Integer) (money :type "Float (double-precision)") (HP :type "Float (double-precision)") (Firepower :type "Float (double-precision)"))
  (set `self.EXP` EXP)
  (set `self.EXP to update` `EXP to update`)
  (set `self.Grade` grade)
  (set `self.EXP 100` `EXP to update`)
  (set `self.Money` money)
  (set `self.HP` HP)
  (set `self.Firepower` Firepower))

(fn `Update number of item1`
  (params (`Use or Pickup` :type Integer))
  (`/Game/UI/UI_state.Update_UI_cell1` (`self.UI_state`) (`/Game/Data_assets/Player_Data_Assets/DA_Character.number1` (`self.Player_data`)) `Use or Pickup`))

(fn `Update number of item2`
  (params (`Use or Pickup` :type Integer))
  (`/Game/UI/UI_state.Update_UI_cell2` (`self.UI_state`) (`/Game/Data_assets/Player_Data_Assets/DA_Character.number2` (`self.Player_data`)) `Use or Pickup`))

(fn `Update number of item3`
  (params (`Use or Pickup` :type Integer))
  (`/Game/UI/UI_state.Update_UI_cell3` (`self.UI_state`) (`/Game/Data_assets/Player_Data_Assets/DA_Character.number3` (`self.Player_data`)) `Use or Pickup`))

(fn `Update_EXP`
  (`/Game/UI/UI_state.Update_EXP` (`self.UI_state`) (`self.EXP`) (`self.EXP to update`))
  (`/Game/UI/UI_state.Update_LV+EXP` (`self.UI_state`) (`self.Grade`) (`self.EXP`) (`self.EXP to update`)))

(fn `Update_EXP_Standard`
  (set `self.EXP to update` (* (`self.EXP 100`) (`KismetMathLibrary.MultiplyMultiply_FloatFloat` (`/Game/Data_assets/Player_Data_Assets/DA_Character.EXP_standard` (`self.Player_data`)) (`KismetMathLibrary.Conv_IntToDouble` (- (`self.Grade`) 1))))))

(fn `Update_HP`
  (`/Game/UI/UI_state.Update_HP` (`self.UI_state`) (`self.HP`) (`/Game/Data_assets/Player_Data_Assets/DA_Character.HPmax` (`self.Player_data`)))
  (`/Game/UI/UI_state.Update_HPprogress` (`self.UI_state`) (`self.HP`) (`/Game/Data_assets/Player_Data_Assets/DA_Character.HPmax` (`self.Player_data`))))

(fn `Use of item`)

(fn `UserConstructionScript`)