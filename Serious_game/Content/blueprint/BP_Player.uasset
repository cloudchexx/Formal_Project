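; BP_Player is the player Blueprint, handling movement and the on-screen status HUD.
; The IA_Move Enhanced Input action drives movement along fixed world X and Y axes, then calls HUDInitialize.
; HUDInitialize creates a UI_state widget, adds it to the viewport and fills its EXP and HP from PlayerData.
; Because it runs from the move event rather than BeginPlay, each firing creates another widget.
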(event `EnhancedInput|/Game/Enhanced_inputs/IA_Move`
  (params (ActionValue :type "Vector2D Structure") (ElapsedSeconds :type "Float (double-precision)") (TriggeredSeconds :type "Float (double-precision)") (InputAction :type "InputAction Object Reference" :default "/Game/Enhanced_inputs/IA_Move.IA_Move"))
  (bind (_x _y) (`KismetMathLibrary.BreakVector2D` ActionValue))
  (:`Triggered`
    (set `self.X` _x)
    (set `self.Y` _y)
    (`self.AddMovementInput` (1.0 0.0 0.0) (`self.X`))
    (`self.AddMovementInput` (0.0 1.0 0.0) (`self.Y`))
    (`self.HUD_initialize`)))

(fn `HUD_initialize`
  (bind _player_data (`self.Player_data`))
  (bind _player_data_2 (`self.Player_data`))
  (bind _returnvalue (`|CreateWidget` "/Game/UI/UI_state.UI_state_C"))
  (bind _output_get (set `self.UI_state` _returnvalue))
  (`UserWidget.AddToViewport` _output_get 0)
  (`/Game/UI/UI_state.Update_EXP` (`self.UI_state`) (`/Game/Data_assets/DA_Character.Experience` _player_data) (`/Game/Data_assets/DA_Character.Experience points required to upgrade` _player_data))
  (`/Game/UI/UI_state.Update_HP` (`self.UI_state`) (`/Game/Data_assets/DA_Character.HP` _player_data_2) (`/Game/Data_assets/DA_Character.HPmax` _player_data_2)))

(fn `UserConstructionScript`)