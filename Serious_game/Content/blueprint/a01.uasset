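; Actor Blueprint a01 with placeholder-named functions and no clear gameplay purpose.
; BeginPlay, overlap and Tick are disabled empty stubs, and the construction script is empty.
; Lll queries actors by class, prints its own display name and spawns an AI, while Ll only runs the query.
; 01111 spawns two AI; nothing in the graphs calls these functions or uses the query results.
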(fn `01111`
  (`AIBlueprintHelperLibrary.SpawnAIFromClass` null null (0.0 0.0 0.0) (struct) false null)
  (`AIBlueprintHelperLibrary.SpawnAIFromClass` null null (0.0 0.0 0.0) (struct) false null)
  (return))

(fn `ll`
  (`GameplayStatics.GetAllActorsOfClass` null))

(fn `lll`
  (`GameplayStatics.GetAllActorsOfClass` null)
  (`KismetSystemLibrary.PrintString` (`KismetSystemLibrary.GetDisplayName` self))
  (`AIBlueprintHelperLibrary.SpawnAIFromClass` null null (0.0 0.0 0.0) (struct) false null))

(fn `UserConstructionScript`)