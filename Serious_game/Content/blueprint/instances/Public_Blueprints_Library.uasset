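; Public Blueprint library of helpers for game instance access and single-slot save and load.
; SAVE GAME creates a fresh SaveGame_Player, passes it the current level name via SaveData and writes it to a hardcoded slot; its existence check is unwired.
; READ GAME opens the saved level if the slot exists, with debug prints reporting results.
; View the archive is an empty stub.
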(fn `get Game_instances`
  (returns (`AsGame Instances` :type "/Game/blueprint/instances/Game_instances Object Reference"))
  ;[1 1 1] get Game instances
  (bind _asgame_instances (cast `/Game/blueprint/instances/Game_instances` (`GameplayStatics.GetGameInstance` null)))
  (return _asgame_instances))

(fn `READ GAME`
  ;[1 1 1] READ GAME
  (bind _returnvalue (`GameplayStatics.DoesSaveGameExist` "0918"))
  (if _returnvalue
    (bind _returnvalue_2 (`GameplayStatics.LoadGameFromSlot` "0918"))
    (bind _assave_game_player (cast `/Game/blueprint/instances/Game_DATA/SaveGame_Player` _returnvalue_2))
    (`GameplayStatics.OpenLevel` null (`KismetStringLibrary.Conv_StringToName` (`/Game/blueprint/instances/Game_DATA/SaveGame_Player.level_name` _assave_game_player)))
    (`KismetSystemLibrary.PrintString` null "ok")
    (else
      (`KismetSystemLibrary.PrintString` null "no DATA"))))

(fn `SAVE GAME`
  (returns (ReturnValue :type Boolean))
  ;[1 1 1] SAVE GAME
  (bind _returnvalue (`GameplayStatics.CreateSaveGameObject` "/Game/blueprint/instances/Game_DATA/SaveGame_Player.SaveGame_Player_C"))
  (bind _returnvalue_2 (`GameplayStatics.GetCurrentLevelName` null))
  (`/Game/blueprint/instances/Game_DATA/SaveGame_Player.Save_Data` _returnvalue _returnvalue_2)
  (bind _returnvalue_3 (`GameplayStatics.SaveGameToSlot` _returnvalue "0918"))
  (`KismetSystemLibrary.PrintString` null "save")
  (return _returnvalue_3))

(fn `View the archive`
  (return))