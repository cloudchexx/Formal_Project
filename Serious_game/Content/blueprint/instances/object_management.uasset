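; Object manager actor that runs an object pool of pickup item props for the game.
; On BeginPlay it registers itself on the game instance's ObjectManagement reference.
; SettingUpPropsPool searches the pool for a prop with a matching status, spawning a Pickup_items below the origin and pooling it if no valid prop results.
; It then calls GenerateAPoolOfProps on that prop and teleports it to the requested location.
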(event `self.ReceiveBeginPlay`
  (set `/Game/blueprint/instances/Game_instances.object management` self (`/Game/blueprint/instances/Public_Blueprints_Library.get Game_instances`)))

(fn `Setting up props pool`
  (params (`Generation location` :type "Vector Structure"))
  (locals (props :type "/Game/Props/Pickup_items Object Reference"))
  ;[1 1 1] Setting up the prop pool
  (for _array_element (`self.props pool`)
    (if (`|EnumEquality` (`/Game/Props/Pickup_items.Status of props` _array_element) "NewEnumerator1")
      (set `local.props` _array_element)
      (break)))
  (`local.props`
    (:`then`
      _)
    (:`else`
      (bind _returnvalue (`|SpawnActorFromClass` "/Game/Props/Pickup_items.Pickup_items_C" (`KismetMathLibrary.MakeTransform` (200.0 200.0 -1000.0)) "Undefined" "MultiplyWithRoot" null null))
      (bind _output_get (set `local.props` _returnvalue))
      (`KismetArrayLibrary.Array_AddUnique` (`self.props pool`) _output_get)))
  (`/Game/Props/Pickup_items.Generate a pool of props` (`local.props`) 10.0)
  (`self.K2_TeleportTo` :`self` (`local.props`) :`DestLocation` (`local.Generation location`)))

(fn `UserConstructionScript`)